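; BP_Door is a door actor that moves vertically according to how many chunks are registered with it.
; AddChunk and RemoveChunk raise or lower the ChunkThreshold counter and compare it to RequiredChunkAmount.
; At or above that amount the DoorMovement timeline plays forward, otherwise it reverses, with its Height track driving the Door component's relative Z location.
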(event Custom|AddChunk
  (bind _result (Math|Integer|IncrementInt (Variables|Default|GetChunkThreshold))
    (:%20%20
      (if (>= _result (Variables|Default|GetRequiredChunkAmount))
        (bind _height (Timeline|DoorMovement Play)
          (:Update
            (Transformation|SetRelativeLocation (Variables|Default|GetDoor) (Math|Vector|MakeVector 0.0 0.0 _height) false false)))
        (else
          (Timeline|DoorMovement Reverse))))))

(event Custom|RemoveChunk
  (bind _result (Math|Integer|DecrementInt (Variables|Default|GetChunkThreshold))
    (:%20%20
      (if (>= _result (Variables|Default|GetRequiredChunkAmount))
        (bind _height (Timeline|DoorMovement Play)
          (:Update
            (Transformation|SetRelativeLocation (Variables|Default|GetDoor) (Math|Vector|MakeVector 0.0 0.0 _height) false false)))
        (else
          (Timeline|DoorMovement Reverse))))))

(fn ConstructionScript)