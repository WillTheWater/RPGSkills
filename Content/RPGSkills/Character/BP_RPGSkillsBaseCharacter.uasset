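; Base character for the RPG skills system, linking the player to the overlay UI and an aiming-style camera.
; It sets and reads the overlay's active widget switcher page through a UI reference.
; Crosshair and camera mode toggles the overlay crosshair and shifts the camera boom between centered and a raised side offset.
; A timeline eases the boom's socket offset toward the target.
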(event Custom|CameraOffset
  (params (CameraTargetOffset :type Vector))
  (bind _cameraboom (Variables|Default|GetCameraBoom))
  (bind _alpha (Timeline|TL_CameraOffset PlayFromStart)
    (:Update
      (Variables|/Script/Engine.SpringArmComponent|SetSocketOffset _cameraboom (Math|Vector|Lerp(Vector) (Variables|/Script/Engine.SpringArmComponent|GetSocketOffset _cameraboom) CameraTargetOffset _alpha)))))

(event EventBeginPlay)

(event Collision|EventActorBeginOverlap
  (params (OtherActor :type Actor%20Object%20Reference)))

(event EventTick
  (params (DeltaSeconds :type Float%20%28single-precision%29)))

(event EventSetWidgetSwitcherIndex
  (params (Index :type Integer))
  (bind _uireference (Variables|Default|GetUIReference)
    (:then
      (bind _aswb_rpgoverlay_ui (Utilities|Casting|CastToWB_RPGOverlayUI _uireference))
      (Class|WidgetSwitcher|SetActiveWidgetIndex (Variables|/Game/RPGSkills/UI/WB_RPGOverlayUI.WB_RPGOverlayUI_C|GetWidgetSwitcher _aswb_rpgoverlay_ui) Index))
    (:else)))

(event EventCrosshairandCameraMode
  (params (bShow :type Boolean))
  (bind _returnvalue (select bShow 45.0 0.0))
  (Utilities|FlowControl|Sequence
    (:then_0
      (bind _uireference (Variables|Default|GetUIReference)
        (:then
          (bind _aswb_rpgoverlay_ui (Utilities|Casting|CastToWB_RPGOverlayUI _uireference))
          (Default|HandleCrosshairDisplay _aswb_rpgoverlay_ui bShow))
        (:else)))
    (:then_1
      (CallFunction|CameraOffset (Math|Vector|MakeVector 0.0 _returnvalue _returnvalue)))))

(fn ConstructionScript)

(fn GetWidgetSwitcherInfo
  (bind _uireference (Variables|Default|GetUIReference)
    (:then
      (bind _aswb_rpgoverlay_ui (Utilities|Casting|CastToWB_RPGOverlayUI _uireference)
        (:then
          (return (Class|WidgetSwitcher|GetActiveWidgetIndex (Variables|/Game/RPGSkills/UI/WB_RPGOverlayUI.WB_RPGOverlayUI_C|GetWidgetSwitcher _aswb_rpgoverlay_ui))))
        (:CastFailed
          (return -1))))
    (:else)))